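; BP_PlayerPawn is a player pawn Blueprint whose only logic is a GetActorList function that finds objects in front of it.
; GetActorList runs a complex multi-sphere trace on the Visibility channel along the forward vector, ignoring itself and drawing timed debug shapes.
; It stores the hit results in FoundObjects and returns them.
; The event graph and construction script are empty, and nothing here calls the function.
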(fn `GetActorList`
  (returns (ReturnValue :type "Array of HitResult Structure"))
  (locals (FoundObjects :type "Array of HitResult Structure"))
  (bind _returnvalue (`self.K2_GetActorLocation` self))
  (bind _returnvalue_2 (`self.GetActorForwardVector` self))
  (bind _outhits (`KismetSystemLibrary.SphereTraceMulti` (+ _returnvalue (* _returnvalue_2 80)) (+ _returnvalue (* _returnvalue_2 160)) 80.0 "TraceTypeQuery1" true (`|MakeArray` self :!type "Actor Object Reference") "ForDuration"))
  (bind _output_get (set `local.FoundObjects` _outhits))
  (return _output_get))

(fn `UserConstructionScript`)